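; Player is a character Blueprint that handles basic player input for looking, moving and jumping.
; Mouse axes drive controller yaw and pitch, and the jump action starts and stops jumping on press and release.
; Movement axes add input along the forward and right vectors of the full control rotation, so pitch is not stripped from the movement direction.
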(event Input|ActionEvents|InputActionaction_jump
  (params (Key :type Key%20Structure :default "None"))
  (:Pressed
    (Character|Jump))
  (:Released
    (Character|StopJumping)))

(event Input|AxisEvents|InputAxisforward_movement
  (params (AxisValue :type Float%20%28single-precision%29))
  ;[1 1 1] Player_Movement
  (Pawn|Input|AddMovementInput (Math|Vector|GetForwardVector (Pawn|GetControlRotation :!class /Script/Engine.Pawn)) AxisValue false))

(event Input|AxisEvents|InputAxisleft_right
  (params (AxisValue :type Float%20%28single-precision%29))
  ;[1 1 1] Player_Movement
  (Pawn|Input|AddMovementInput (Math|Vector|GetRightVector (Pawn|GetControlRotation :!class /Script/Engine.Pawn)) AxisValue false))

(event Input|AxisEvents|InputAxismouse_right
  (params (AxisValue :type Float%20%28single-precision%29))
  ;[1 1 1] mouse_controller
  (Pawn|Input|AddControllerYawInput AxisValue))

(event Input|AxisEvents|InputAxismouse_up
  (params (AxisValue :type Float%20%28single-precision%29))
  ;[1 1 1] mouse_controller
  (Pawn|Input|AddControllerPitchInput AxisValue))

(fn ConstructionScript)